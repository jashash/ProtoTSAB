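; BP_TrainingMode sets up the player's character when the training mode begins play.
; On BeginPlay it passes every PlayerStart to SpawnPlayers, which acts only on those tagged "P1".
; DetermineCharacterClass spawns a Dummy or SMG character at that start, based on the CharacterClass stored in BaseGameInstance.
; The spawned character is saved as Player1 and possessed by player controller 0.
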(event `self.ReceiveBeginPlay`
  (bind _outactors (`GameplayStatics.GetAllActorsOfClass` "/Script/Engine.PlayerStart"))
  (for _array_element _outactors
    (`self.SpawnPlayers` _array_element)))

(fn `DetermineCharacterClass`
  (params (Transform :type "Transform Structure") (Actor :type "Actor Object Reference"))
  (returns (retval :type "PlayerCharacter Object Reference"))
  (bind _asbase_game_instance (cast `BaseGameInstance` (`GameplayStatics.GetGameInstance`)))
  (switch `ECharacter` (`BaseGameInstance.characterClass` _asbase_game_instance)
    (:`VE_Default`
      (bind _returnvalue (`|SpawnActorFromClass` "/Game/Blueprints/BP_Dummy.BP_Dummy_C" Transform "Undefined" "OverrideRootScale" Actor null))
      (return _returnvalue))
    (:`VE_SMG`
      (bind _returnvalue_2 (`|SpawnActorFromClass` "/Game/Blueprints/BP_SMG.BP_SMG_C" Transform "Undefined" "OverrideRootScale" Actor null))
      (return _returnvalue_2))))

(fn `SpawnPlayers`
  (params (Object :type "Actor Object Reference"))
  (bind _asplayer_start (cast `PlayerStart` Object))
  (if (== (`PlayerStart.PlayerStartTag` _asplayer_start) "P1")
    (bind _retval (`self.DetermineCharacterClass` (`self.GetTransform` Object) Object))
    (set `self.player1` _retval)
    (`Controller.Possess` (`GameplayStatics.GetPlayerController` 0) _retval)))

(fn `UserConstructionScript`)