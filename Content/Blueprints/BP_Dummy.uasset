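; BP_Dummy is a dummy actor that displays a health bar through a widget component.
; On BeginPlay it caches the BP_HealthBar widget, then sets a fixed world rotation on the component and makes that rotation absolute, so it ignores parent rotation.
; Every Tick it pushes HealthPercent into the progress bar; the graph shows no damage handling or other logic that changes that value.
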(event `self.ReceiveBeginPlay`
  (bind _healthbar (`self.HealthBar`))
  (bind _asbp_health_bar (cast `/Game/Blueprints/Widgets/BP_HealthBar` (`WidgetComponent.GetUserWidgetObject` (`self.HealthBar`))))
  (set `self.HealthBarUIRef` _asbp_health_bar)
  (`SceneComponent.K2_SetWorldRotation` _healthbar (struct :`Pitch` 70.0) false false)
  (set `SceneComponent.bAbsoluteRotation` true _healthbar))

(event `self.ReceiveTick`
  (params (DeltaSeconds :type "Float (single-precision)"))
  (`ProgressBar.SetPercent` (`/Game/Blueprints/Widgets/BP_HealthBar.HealthBar` (`self.HealthBarUIRef`)) (`self.HealthPercent`)))

(fn `UserConstructionScript`)